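; BP_MobileCube1_Auto2 is a movable physics cube with its own switchable gravity direction.
; Every tick it applies a mass-independent force along the current direction from the DTGravityDIr table.
; A global gravity event from BPGB sets that direction, while interaction input scales velocity by the current direction vector, then cycles through seven entries.
; An Axis component starts hidden and holds zero world rotation during interaction.
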(event Custom|SetSelfGravity
  (params (GravityDir :type Integer))
  (Variables|Default|SetNowDir GravityDir))

(event EventOnInteractOtherInput
  ;[0.15 0.15 0.15 0.5] 设置重力方向
  (Physics|SetPhysicsLinearVelocity (Variables|Default|GetCube) (* (Transformation|GetVelocity) (Utilities|Array|Get(acopy) (Variables|/Game/LevelPrototyping/Interactable/Data/DT_GravityDIr.DT_GravityDIr_C|GetGravityDir (Variables|Default|GetDT_GravityDIr)) (Variables|Default|GetNowDir))) false "None")
  (Variables|Default|SetNowDir (Math|Integer|%(Integer) (+ (Variables|Default|GetNowDir) 1) 7)))

(event EventTick
  (params (DeltaSeconds :type Float%20%28single-precision%29))
  ;[0.15 0.15 0.15 0.5] 施加重力
  (Physics|AddForce (Variables|Default|GetCube) (* (Utilities|Array|Get(acopy) (Variables|/Game/LevelPrototyping/Interactable/Data/DT_GravityDIr.DT_GravityDIr_C|GetGravityDir (Variables|Default|GetDT_GravityDIr)) (Variables|Default|GetNowDir)) 1e+03) "None" true)
  (if (Variables|Default|GetIsInteracting)
    (Transformation|SetWorldRotation (Variables|Default|GetAxis) "0, 0, 0" false false)))

(event EventBeginPlay
  ;[0.15 0.15 0.15 0.5] 初始化可见性和重力方向
  (Rendering|SetVisibility (Variables|Default|GetAxis) false false)
  (EventDispatchers|BindEventtoEDSetGlobalGravity (Variables|Default|GetBP_GB) (delegate Custom|SetSelfGravity)))

(fn ConstructionScript)