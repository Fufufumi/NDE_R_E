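; BP_MobileCube_T1 is an interactable physics cube with switchable gravity direction and a weight value.
; Each Tick applies mass-independent acceleration along the current direction, which gravity events update.
; Pressing E toggles interaction and a world-aligned axis display, while other functions report weight and test it against pressure-panel thresholds.
; Weight-based coloring, random angular damping and global gravity dispatcher binding are unwired, so never run.
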(event Custom|SetGlobalGravity
  (params (GravityDir :type Integer))
  ;[0.15 0.15 0.15 0.5] 绑定全局事件
  (Variables|Default|SetNowDir GravityDir))

(event EventChInteractSetGravityDir
  (params (GravityDir :type Integer))
  (Variables|Default|SetNowDir GravityDir))

(event EventTick
  (params (DeltaSeconds :type Float%20%28single-precision%29))
  ;[0.15 0.15 0.15 0.5] 施加重力
  (Physics|AddForce (Variables|Default|GetCube) (* (Utilities|Array|Get(acopy) (Variables|/Game/LevelPrototyping/Interactable/Data/DT_GravityDIr.DT_GravityDIr_C|GetGravityDir (Variables|Default|GetDT_GravityDIr)) (Variables|Default|GetNowDir)) 1e+03) "None" true)
  (if (Variables|Default|GetIsInteracting)
    (Transformation|SetWorldRotation (Variables|Default|GetAxis) "0, 0, 0" false false)))

(event EventBeginPlay
  ;[0.15 0.15 0.15 0.5] 初始化可见性和重力方向
  (Rendering|SetVisibility (Variables|Default|GetAxis) false false))

(fn ConstructionScript)

(fn ChInteract
  (params (Interactor :type Actor%20Object%20Reference) (PressedKey :type Key%20Structure) (RmbPressed :type Boolean))
  (if (== PressedKey "E")
    (bind _output_get (Variables|Default|SetIsInteracting (not (Variables|Default|GetIsInteracting))))
    (Rendering|SetVisibility (Variables|Default|GetAxis) _output_get false)
    (return (Variables|Default|GetCube) true true)))

(fn GravitySend
  (return (Variables|Default|GetTheM)))

(fn PressurepanelFunc
  (params (MIn :type Integer))
  (return (<= MIn (Variables|Default|GetTheM))))